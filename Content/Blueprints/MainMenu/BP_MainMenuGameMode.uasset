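; Game mode for the main menu level that manages which menu screen is shown.
; On BeginPlay it switches the player to game-and-UI input, shows the mouse cursor and opens the main menu.
; Two functions switch between the MainMenu and BrowseMenu widgets, each removing all existing widgets before creating and adding a fresh one to the viewport.
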(event `self.ReceiveBeginPlay`
  (bind _returnvalue (`GameplayStatics.GetPlayerController` 0))
  (`WidgetBlueprintLibrary.SetInputMode_GameAndUIEx` _returnvalue)
  (set `PlayerController.bShowMouseCursor` true _returnvalue)
  (`self.AddMainMenuWidget`))

(fn `AddBrowseMenuWidget`
  (`WidgetLayoutLibrary.RemoveAllWidgets`)
  (bind _returnvalue (`|CreateWidget` "/Game/UMG/BrowseMenu.BrowseMenu_C" (`GameplayStatics.GetPlayerController` 0)))
  (`UserWidget.AddToViewport` _returnvalue 0))

(fn `AddMainMenuWidget`
  (`WidgetLayoutLibrary.RemoveAllWidgets`)
  (bind _returnvalue (`|CreateWidget` "/Game/UMG/MainMenu.MainMenu_C" (`GameplayStatics.GetPlayerController` 0)))
  (`UserWidget.AddToViewport` _returnvalue 0))

(fn `UserConstructionScript`)