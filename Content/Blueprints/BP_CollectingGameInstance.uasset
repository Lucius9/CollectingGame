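; A game instance Blueprint for the collecting game that reports network failures to the player.
; It handles the network error event by mapping each failure type to a readable message string.
; It then creates a NetWorkError widget for the first local player with that message and adds it to the viewport.
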(event `self.HandleNetworkError`
  (params (FailureType :type "ENetworkFailure Enum" :default "NetDriverAlreadyExists") (bIsServer :type Boolean))
  (switch `ENetworkFailure` FailureType
    (:`NetDriverAlreadyExists`
      (set `self.ErrorMessage` "A relevant net driver has already been created for this service"))
    (:`NetDriverCreateFailure`
      (set `self.ErrorMessage` "The net driver creation failed"))
    (:`NetDriverListenFailure`
      (set `self.ErrorMessage` "The net driver failed its Listen() call "))
    (:`ConnectionLost`
      (set `self.ErrorMessage` "A connection to the net driver has been lost"))
    (:`ConnectionTimeout`
      (set `self.ErrorMessage` "A connection to the net driver has timed out"))
    (:`FailureReceived`
      (set `self.ErrorMessage` "The net driver received an NMT_Failure message "))
    (:`OutdatedClient`
      (set `self.ErrorMessage` "The client needs to upgrade their game"))
    (:`OutdatedServer`
      (set `self.ErrorMessage` "The server needs to upgrade their game "))
    (:`PendingConnectionFailure`
      (set `self.ErrorMessage` "There was an error during connection to the game"))
    (:`NetGuidMismatch`
      (set `self.ErrorMessage` "NetGuid mismatch"))
    (:`NetChecksumMismatch`
      (set `self.ErrorMessage` "Network checksum mismatch")))
  (bind _returnvalue (`|CreateWidget` "/Game/UMG/NetWorkError.NetWorkError_C" (`GameplayStatics.GetPlayerController` 0) (`self.ErrorMessage`)))
  (`UserWidget.AddToViewport` _returnvalue 0))